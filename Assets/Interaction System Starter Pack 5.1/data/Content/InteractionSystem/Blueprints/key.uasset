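; A key pickup in the interaction system that spins continuously and unlocks the Box matching its KeyIndex.
; Tick rotates the Sphere around its yaw axis.
; When a Character overlaps Sphere1, the key loops over all Box actors until BoxIndex equals KeyIndex, sets CanOpen on that element, and destroys itself.
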(event `self.ReceiveTick`
  (params (DeltaSeconds :type "Float (single-precision)"))
  ;[1 1 1] SelfRotation
  (`SceneComponent.K2_AddWorldRotation` (`self.Sphere`) (`KismetMathLibrary.MakeRotator` 0.0 0.0 (* DeltaSeconds 360.0)) false false))

(event `self.Sphere1.OnComponentBeginOverlap`
  (params (OverlappedComponent :type "PrimitiveComponent Object Reference") (OtherActor :type "Actor Object Reference") (OtherComp :type "PrimitiveComponent Object Reference") (OtherBodyIndex :type Integer) (bFromSweep :type Boolean) (SweepResult :type "HitResult Structure (by ref)"))
  ;[1 0 0.6621] 更换你的角色蓝图
  (cast `Character` OtherActor)
  (bind _outactors (`GameplayStatics.GetAllActorsOfClass` "/Game/InteractionSystem/Blueprints/Box.Box_C"))
  (for _array_element _outactors
    (if (== (`/Game/InteractionSystem/Blueprints/Box.BoxIndex` _array_element) (`self.KeyIndex`))
      (break)))
  (set `/Game/InteractionSystem/Blueprints/Box.CanOpen?` true _array_element)
  (`self.K2_DestroyActor`))

(fn `UserConstructionScript`)