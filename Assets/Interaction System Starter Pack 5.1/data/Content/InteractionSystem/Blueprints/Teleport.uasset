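; Teleport pad actor that moves a Character entering its Box to another Teleport actor sharing the same TeleportIndex.
; On overlap, if Can is set, it searches all Teleport actors for the first other match and places the character at that actor's Scene component location with zeroed velocity.
; The destination's Can flag is switched off for a one-second delay to prevent an immediate bounce back.
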(event `self.Box.OnComponentBeginOverlap`
  (params (OverlappedComponent :type "PrimitiveComponent Object Reference") (OtherActor :type "Actor Object Reference") (OtherComp :type "PrimitiveComponent Object Reference") (OtherBodyIndex :type Integer) (bFromSweep :type Boolean) (SweepResult :type "HitResult Structure (by ref)"))
  (if (`self.Can`)
    (bind _ascharacter (cast `Character` OtherActor))
    (bind _outactors (`GameplayStatics.GetAllActorsOfClass` "Teleport_C"))
    (for _array_element _outactors
      (if (== _array_element self)
        _
        (elif (== (`/Game/InteractionSystem/Blueprints/Teleport.TeleportIndex` _array_element) (`self.TeleportIndex`))
          (break))))
    (set `/Game/InteractionSystem/Blueprints/Teleport.Can` false _array_element)
    (`self.K2_SetActorLocation` _ascharacter (`SceneComponent.K2_GetComponentLocation` (`/Game/InteractionSystem/Blueprints/Teleport.Scene` _array_element)) false true)
    (set `MovementComponent.Velocity` (0.0 0.0 0.0) (`Character.CharacterMovement` _ascharacter))
    (`KismetSystemLibrary.Delay` 1.0)
    (set `/Game/InteractionSystem/Blueprints/Teleport.Can` true _array_element)))

(fn `UserConstructionScript`)